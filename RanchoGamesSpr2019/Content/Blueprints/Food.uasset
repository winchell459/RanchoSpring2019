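; Food pickup for a snake-style game that grows the player's tail when Player_BP overlaps its collision.
; On overlap it spawns a PlayerTail_BP_2 at the current tail and sets that tail as its head.
; Segments form a linked list: the new one becomes NextLink of the player or last segment, then MyTail.
; The food then moves to a random point on the XZ plane instead of being destroyed.
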(event OnComponentBeginOverlap(Collision)
  (params (OverlappedComponent :type Primitive%20Component%20Object%20Reference) (OtherActor :type Actor%20Object%20Reference) (OtherComp :type Primitive%20Component%20Object%20Reference) (OtherBodyIndex :type Integer) (bFromSweep :type Boolean) (SweepResult :type Hit%20Result%20Structure%20%28by%20ref%29))
  (bind _asplayer_bp (Utilities|Casting|CastToPlayer_BP OtherActor))
  (bind _output_get (Variables|Default|SetPlayer _asplayer_bp))
  (bind _returnvalue (Game|SpawnActorfromClass "/Game/Blueprints/PlayerTail_BP_2.PlayerTail_BP_2_C" (Transformation|GetActorTransform (Variables|/Game/Blueprints/Player_BP.Player_BP_C|GetMyTail _output_get)) "Undefined" 0 0))
  (Default|SetHead _returnvalue (Variables|/Game/Blueprints/Player_BP.Player_BP_C|GetMyTail _output_get))
  (if (== (Variables|/Game/Blueprints/Player_BP.Player_BP_C|GetNextLink (Variables|Default|GetPlayer)) (Variables|Default|GetPlayer))
    (Variables|/Game/Blueprints/Player_BP.Player_BP_C|SetNextLink (Variables|Default|GetPlayer) _returnvalue)
    (else
      (bind _asplayer_tail_bp_2 (Utilities|Casting|CastToPlayerTail_BP_2 (Variables|/Game/Blueprints/Player_BP.Player_BP_C|GetMyTail _output_get)))
      (Variables|/Game/Blueprints/PlayerTail_BP_2.PlayerTail_BP_2_C|SetNextLink _asplayer_tail_bp_2 _returnvalue)))
  (Variables|/Game/Blueprints/Player_BP.Player_BP_C|SetMyTail (Variables|Default|GetPlayer) _returnvalue)
  (Transformation|SetActorTransform (Math|Transform|MakeTransform (Math|Vector|MakeVector (Math|Random|RandomFloatinRange -2e+02 1e+03) 0.0 (Math|Random|RandomFloatinRange 2e+02 1.35e+03)))))

(fn ConstructionScript)