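; PlayerTail_BP is a tail link in a player-following chain, computing its movement on the X-Z plane toward CurrentTarget.
; Tick caches DeltaSeconds, and CalcDisplacement derives DeltaMove from PlayerSpeed, stopping within Buffer when FollowingParent.
; When its distance-scaled step would overshoot, it zeroes movement and hands the first queued NextTarget point down to NextLink.
; The graph only calculates DeltaMove and never applies it to the actor.
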(event Custom|CalcDisplacement
  (bind _returnvalue (Transformation|GetActorLocation))
  (bind _currenttarget (Variables|Default|GetCurrentTarget))
  (bind _nexttarget (Variables|Default|GetNextTarget))
  ;[1 1 1] Calc Displacment
  (bind _output_get (Variables|Default|SetPlayerDisplacement (Math|Vector|MakeVector (- (.x _currenttarget) (.x _returnvalue)) 0.0 (- (.z _currenttarget) (.z _returnvalue)))))
  (if (>= (Math|Vector|VectorLength (* (Math|Vector|Normalize _output_get) (* (Variables|Default|GetPlayerSpeed) (Variables|Default|GetDeltaSeconds) (Math|Vector|VectorLength _output_get)))) (Math|Vector|VectorLength _output_get))
    (Variables|Default|SetDeltaMove (* (Math|Vector|Normalize _output_get) (* (Variables|Default|GetPlayerSpeed) (Variables|Default|GetDeltaSeconds) (Math|Vector|VectorLength _output_get))))
    (if (> (Utilities|Array|Length (Variables|Default|GetNextTarget)) 0)
      (bind _asplayer_tail_bp (Utilities|Casting|CastToPlayerTail_BP (Variables|Default|GetNextLink))
        (:then
          (Utilities|Array|Add (Variables|PlayerTail_BP_C|GetNextTarget _asplayer_tail_bp) (Utilities|Array|Get(acopy) _nexttarget)))
        (:CastFailed
          _))
      (Utilities|Array|RemoveIndex _nexttarget)
      (bind _output_get_2 (Variables|Default|SetPlayerDisplacement "0, 0, 0"))
      (Variables|Default|SetDeltaMove _output_get_2)
      (else
        (bind _output_get_3 (Variables|Default|SetPlayerDisplacement "0, 0, 0" :!label _label))
        (Variables|Default|SetDeltaMove _output_get_3)))
    (else
      (if (Variables|Default|GetFollowingParent)
        (if (< (Math|Vector|VectorLength (Variables|Default|GetPlayerDisplacement)) (Variables|Default|GetBuffer))
          (goto _label)
          (else
            _)))
      (Variables|Default|SetDeltaMove (* (Math|Vector|Normalize (Variables|Default|GetPlayerDisplacement)) (* (Variables|Default|GetPlayerSpeed) (Variables|Default|GetDeltaSeconds)))))))

(event EventTick
  (params (DeltaSeconds :type Float%20%28single-precision%29))
  (Variables|Default|SetDeltaSeconds DeltaSeconds))

(fn ConstructionScript)