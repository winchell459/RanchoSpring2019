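; Tail segment actor that trails the actor set through SetHead, forming a chain of links.
; Each tick it steps at PlayerSpeed in the XZ plane toward the first queued waypoint, or toward the followed actor when none are queued.
; Reached waypoints are removed and passed to the next PlayerTail_BP_2 link, so segments retrace the same path.
; When following the actor directly, it halts within a Buffer distance.
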(event Custom|CalcDisplacment
  (bind _returnvalue (Transformation|GetActorLocation))
  (bind _currenttarget (Variables|Default|GetCurrentTarget))
  (bind _nexttarget (Variables|Default|GetNextTarget))
  (bind _output_get (Variables|Default|SetPlayerDisplacement (Math|Vector|MakeVector (- (.x _currenttarget) (.x _returnvalue)) 0.0 (- (.z _currenttarget) (.z _returnvalue)))))
  (if (>= (Math|Vector|VectorLength (* (Math|Vector|Normalize _output_get) (* (Variables|Default|GetPlayerSpeed) (Variables|Default|GetDeltaTime)))) (Math|Vector|VectorLength _output_get))
    (Variables|Default|SetDeltaMove (* (Math|Vector|Normalize _output_get) (* (Variables|Default|GetPlayerSpeed) (Variables|Default|GetDeltaTime))))
    (if (> (Utilities|Array|Length (Variables|Default|GetNextTarget)) 0)
      (bind _asplayer_tail_bp_2 (Utilities|Casting|CastToPlayerTail_BP_2 (Variables|Default|GetNextLink))
        (:then
          (Utilities|Array|Add (Variables|PlayerTail_BP_2_C|GetNextTarget _asplayer_tail_bp_2) (Utilities|Array|Get(acopy) _nexttarget)))
        (:CastFailed
          _))
      (Utilities|Array|RemoveIndex _nexttarget)
      (bind _output_get_2 (Variables|Default|SetPlayerDisplacement "0, 0, 0"))
      (Variables|Default|SetDeltaMove _output_get_2)
      (else
        (bind _output_get_3 (Variables|Default|SetPlayerDisplacement "0, 0, 0" :!label _label))
        (Variables|Default|SetDeltaMove _output_get_3)))
    (else
      (if (Variables|Default|GetFollowingParent)
        (if (< (Math|Vector|VectorLength (Variables|Default|GetPlayerDisplacement)) (Variables|Default|GetBuffer))
          (goto _label)
          (else
            _)))
      (Variables|Default|SetDeltaMove (* (Math|Vector|Normalize (Variables|Default|GetPlayerDisplacement)) (* (Variables|Default|GetPlayerSpeed) (Variables|Default|GetDeltaTime)))))))

(event EventBeginPlay)

(event Collision|EventActorBeginOverlap
  (params (OtherActor :type Actor%20Object%20Reference)))

(event EventTick
  (params (DeltaSeconds :type Float%20%28single-precision%29))
  (bind _nexttarget (Variables|Default|GetNextTarget))
  (bind _returnvalue (Utilities|Array|Length _nexttarget))
  (bind _returnvalue_2 (> _returnvalue 0))
  (Variables|Default|SetDeltaTime DeltaSeconds)
  (Variables|Default|SetFollowingParent (not _returnvalue_2))
  (if _returnvalue_2
    (Variables|Default|SetCurrentTarget (Utilities|Array|Get(acopy) _nexttarget))
    (else
      (Variables|Default|SetCurrentTarget (Transformation|GetActorLocation (Variables|Default|GetMyFollow)))))
  (CallFunction|CalcDisplacment)
  (Transformation|SetActorTransform (Math|Transform|MakeTransform (+ (Variables|Default|GetDeltaMoveBack) (Variables|Default|GetDeltaMove) (Transformation|GetActorLocation)))))

(fn ConstructionScript)

(fn SetHead
  (params (NewParam :type Pawn%20Object%20Reference))
  (Variables|Default|SetMyFollow NewParam))

(fn SetNextFollow
  (params (nextFollowing :type Pawn%20Object%20Reference))
  (Variables|Default|SetNextLink nextFollowing))