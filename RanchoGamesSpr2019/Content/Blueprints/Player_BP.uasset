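; Player head for a snake-style game that moves continuously along the X-Z plane in the last direction pressed.
; Axis inputs set one of four direction flags and a pitch rotation, which Tick applies with a frame-scaled, unswept transform.
; Each direction change appends the current location to the linked PlayerTail_BP_2's target list as a waypoint.
; Overlapping anything except Food adds a reverse offset to movement until the overlap ends.
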(event OnComponentBeginOverlap(Collision)
  (params (OverlappedComponent :type Primitive%20Component%20Object%20Reference) (OtherActor :type Actor%20Object%20Reference) (OtherComp :type Primitive%20Component%20Object%20Reference) (OtherBodyIndex :type Integer) (bFromSweep :type Boolean) (SweepResult :type Hit%20Result%20Structure%20%28by%20ref%29))
  ;[1 1 1] Collisions
  (Utilities|Casting|CastToFood OtherActor
    (:CastFailed
      (Variables|Default|SetDeltaMoveBack (* (Variables|Default|GetDeltaMove) -1.5)))))

(event OnComponentEndOverlap(Collision)
  (params (OverlappedComponent :type Primitive%20Component%20Object%20Reference) (OtherActor :type Actor%20Object%20Reference) (OtherComp :type Primitive%20Component%20Object%20Reference) (OtherBodyIndex :type Integer))
  ;[1 1 1] Collisions
  (Variables|Default|SetDeltaMoveBack "0, 0, 0"))

(event Custom|CreateWaypoint
  (bind _asplayer_tail_bp_2 (Utilities|Casting|CastToPlayerTail_BP_2 (Variables|Default|GetNextLink)))
  (Utilities|Array|Add (Variables|/Game/Blueprints/PlayerTail_BP_2.PlayerTail_BP_2_C|GetNextTarget _asplayer_tail_bp_2) (Transformation|GetActorLocation)))

(event EventBeginPlay)

(event Collision|EventActorBeginOverlap
  (params (OtherActor :type Actor%20Object%20Reference)))

(event EventTick
  (params (DeltaSeconds :type Float%20%28single-precision%29))
  (bind _playerspeed (Variables|Default|GetPlayerSpeed))
  ;[1 1 1] Movement
  (if (Variables|Default|GetMovingUp)
    (bind _output_get (Variables|Default|SetDeltaMove (Math|Vector|MakeVector 0.0 0.0 (* DeltaSeconds _playerspeed 1.0))))
    (Variables|Default|SetDirection _output_get)
    (Transformation|SetActorTransform (Math|Transform|MakeTransform (+ (Variables|Default|GetDeltaMoveBack) (Variables|Default|GetDirection) (Transformation|GetActorLocation)) (Math|Rotator|MakeRotator 0.0 (Variables|Default|GetPlayerRotation) 0.0)) :!label _label)
    (elif (Variables|Default|GetMovingDown)
      (bind _output_get_2 (Variables|Default|SetDeltaMove (Math|Vector|MakeVector 0.0 0.0 (* DeltaSeconds _playerspeed -1.0))))
      (Variables|Default|SetDirection _output_get_2)
      (goto _label)
      (elif (Variables|Default|GetMovingRight)
        (bind _output_get_3 (Variables|Default|SetDeltaMove (Math|Vector|MakeVector (* DeltaSeconds _playerspeed 1.0) 0.0 0.0)))
        (Variables|Default|SetDirection _output_get_3)
        (goto _label)
        (elif (Variables|Default|GetMovingLeft)
          (bind _output_get_4 (Variables|Default|SetDeltaMove (Math|Vector|MakeVector (* DeltaSeconds _playerspeed -1.0) 0.0 0.0)))
          (Variables|Default|SetDirection _output_get_4)
          (goto _label))))))

(event Input|AxisEvents|InputAxisHorizontal
  (params (AxisValue :type Float%20%28single-precision%29))
  ;[1 1 1] Get Inputs
  (bind _output_get (Variables|Default|SetHorizontalMove AxisValue))
  (if (> _output_get 0.0)
    (if (Variables|Default|GetMovingRight)
      _
      (else
        (CallFunction|CreateWaypoint)))
    (Variables|Default|SetMovingRight true)
    (Variables|Default|SetMovingLeft false)
    (Variables|Default|SetMovingUp false)
    (Variables|Default|SetMovingDown false)
    (Variables|Default|SetPlayerRotation 0.0)
    (elif (< _output_get 0.0)
      (if (Variables|Default|GetMovingLeft)
        _
        (else
          (CallFunction|CreateWaypoint)))
      (Variables|Default|SetMovingRight false)
      (Variables|Default|SetMovingLeft true)
      (Variables|Default|SetMovingUp false)
      (Variables|Default|SetMovingDown false)
      (Variables|Default|SetPlayerRotation 1.8e+02))))

(event Input|AxisEvents|InputAxisVertical
  (params (AxisValue :type Float%20%28single-precision%29))
  ;[1 1 1] Get Inputs
  (bind _output_get (Variables|Default|SetVerticalMove AxisValue))
  (if (> _output_get 0.0)
    (if (Variables|Default|GetMovingUp)
      _
      (else
        (CallFunction|CreateWaypoint)))
    (Variables|Default|SetMovingRight false)
    (Variables|Default|SetMovingLeft false)
    (Variables|Default|SetMovingUp true)
    (Variables|Default|SetMovingDown false)
    (Variables|Default|SetPlayerRotation 9e+01)
    (elif (< _output_get 0.0)
      (if (Variables|Default|GetMovingDown)
        _
        (else
          (CallFunction|CreateWaypoint)))
      (Variables|Default|SetMovingRight false)
      (Variables|Default|SetMovingLeft false)
      (Variables|Default|SetMovingUp false)
      (Variables|Default|SetMovingDown true)
      (Variables|Default|SetPlayerRotation 2.7e+02))))

(fn ConstructionScript)